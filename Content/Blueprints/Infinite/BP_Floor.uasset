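; BP_Floor is a pooled floor segment for an endless level that extends along negative Y and spawns walls ahead of the player.
; Its Box overlap fires once, recycling the previous floor and its walls, then pulling the next floor from the pool and linking back to itself.
; BeginTrace and EndTrace overlaps start and stop a looping timer that spawns BP_Wall from its pool at random preset heights.
; Recycling re-arms the one-shot trigger for reuse.
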(event `self.ReceiveBeginPlay`
  (bind _outactors (`GameplayStatics.GetAllActorsOfClass` "/Game/Blueprints/Infinite/BP_ObjectPoolManager.BP_ObjectPoolManager_C"))
  (for _array_element _outactors
    (if (== (`ObjectPoolManger.ObjectClass` _array_element) "/Game/Blueprints/Infinite/BP_Wall.BP_Wall_C")
      (set `self.Wall_Pool` _array_element)
      (break))))

(event `self.Box.OnComponentBeginOverlap`
  (params (OverlappedComponent :type "PrimitiveComponent Object Reference") (OtherActor :type "Actor Object Reference") (OtherComp :type "PrimitiveComponent Object Reference") (OtherBodyIndex :type Integer) (bFromSweep :type Boolean) (SweepResult :type "HitResult Structure (by ref)"))
  (bind (_returnvalue_x _returnvalue_y _returnvalue_z) (`KismetMathLibrary.BreakVector` (`self.K2_GetActorLocation`)))
  (bind _lastfloor (`self.LastFloor`))
  (`KismetSystemLibrary.PrintString` (`KismetStringLibrary.Concat_StrStr` (`KismetSystemLibrary.GetDisplayName` self) "---" (`KismetSystemLibrary.GetDisplayName` OtherActor)))
  (`/Engine/EditorBlueprintResources/StandardMacros.DoOnce` false :!label _label
    (:`Completed`
      (`/Engine/EditorBlueprintResources/StandardMacros.IsValid` _lastfloor
        (:`Is Valid`
          (`self.DestroyWall` _lastfloor))
        (:`Is Not Valid`
          _))
      (bind _returnvalue (`self.SpawnActorFromPool` (`self.GetOwningPool`) (`KismetMathLibrary.MakeTransform` (`KismetMathLibrary.MakeVector` _returnvalue_x (- _returnvalue_y 4000.0) _returnvalue_z)) "AlwaysSpawn"))
      (bind _asbp_floor (cast `/Game/Blueprints/Infinite/BP_Floor` _returnvalue))
      (set `/Game/Blueprints/Infinite/BP_Floor.LastFloor` self _asbp_floor))))

(event `Resetoverlap`
  (goto _label :!via `Reset`))

(event `self.BeginTrace.OnComponentBeginOverlap`
  (params (OverlappedComponent :type "PrimitiveComponent Object Reference") (OtherActor :type "Actor Object Reference") (OtherComp :type "PrimitiveComponent Object Reference") (OtherBodyIndex :type Integer) (bFromSweep :type Boolean) (SweepResult :type "HitResult Structure (by ref)"))
  (bind _returnvalue (`KismetSystemLibrary.K2_SetTimerDelegate` (delegate `SpawnWall`) 1.0 true)))

(event `DestroyWall`
  ;[1 1 1] 销毁当前地板管理的墙面。
  (for _array_element (`self.SaveWall`)
    (`/Engine/EditorBlueprintResources/StandardMacros.IsValid` _array_element
      (:`Is Valid`
        (`self.PushObjectInPool` _array_element))))
  (`self.PushObjectInPool`)
  (`self.Resetoverlap`))

(event `self.EndTrace.OnComponentBeginOverlap`
  (params (OverlappedComponent :type "PrimitiveComponent Object Reference") (OtherActor :type "Actor Object Reference") (OtherComp :type "PrimitiveComponent Object Reference") (OtherBodyIndex :type Integer) (bFromSweep :type Boolean) (SweepResult :type "HitResult Structure (by ref)"))
  (`KismetSystemLibrary.K2_ClearAndInvalidateTimerHandle` (stale `self.BeginTrace.OnComponentBeginOverlap` _returnvalue)))

(event `SpawnWall`
  (bind _wall_pool (`self.Wall_Pool`))
  (bind (_returnvalue_x _returnvalue_y) (`KismetMathLibrary.BreakVector` (`self.K2_GetActorLocation` (`GameplayStatics.GetPlayerCharacter` 0))))
  (`/Engine/EditorBlueprintResources/StandardMacros.IsValid` _wall_pool
    (:`Is Valid`
      (bind _returnvalue (`self.SpawnActorFromPool` _wall_pool (`KismetMathLibrary.MakeTransform` (`KismetMathLibrary.MakeVector` _returnvalue_x (- _returnvalue_y 600.0) (select `int` (`KismetMathLibrary.RandomInteger` 3) :`0` 90.0 :`1` 200.0 :`2` 150.0 :!type "Float (single-precision)"))) "AlwaysSpawn"))
      (bind _asbp_wall (cast `/Game/Blueprints/Infinite/BP_Wall` _returnvalue))
      (`KismetArrayLibrary.Array_AddUnique` (`self.SaveWall`) _asbp_wall))))

(event `SimpleObjectPoolInterface.BP_PopObject`
  (`KismetSystemLibrary.PrintString` "蓝图Pop" true true (struct :`G` 0.66 :`B` 1.0 :`A` 1.0) 5.0))

(event `SimpleObjectPoolInterface.BP_PushObject`
  (`KismetSystemLibrary.PrintString` "蓝图Push" true true (struct :`G` 0.66 :`B` 1.0 :`A` 1.0) 5.0))

(event `SimpleObjectPoolInterface.BP_ObjectPreinitialized`)

(fn `UserConstructionScript`)