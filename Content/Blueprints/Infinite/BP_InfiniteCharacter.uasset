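; Player character for the Infinite levels that runs automatically in a fixed direction once it has first landed.
; The MoveRight axis event ignores its input value and applies constant movement along world -Y while Start is set.
; Left mouse plays the attack montage and toggles IsAttack on the cached InfiniteLevels_AnimBP until the montage completes.
; Holding Space crouches the character.
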(event `self.ReceiveBeginPlay`
  ;[1 1 1] 游戏开始与移动
  (bind _asinfinite_levels_anim_bp (cast `/Game/Anim/InfiniteLevels_AnimBP` (`SkeletalMeshComponent.GetAnimInstance` (`self.Mesh`))))
  (set `self.AnimInstance` _asinfinite_levels_anim_bp))

(event `self.OnLanded`
  (params (Hit :type "HitResult Structure (by ref)"))
  ;[1 1 1] 游戏开始与移动
  (`/Engine/EditorBlueprintResources/StandardMacros.DoOnce` false
    (:`Completed`
      (set `self.Start` true))))

(event `InputAxis|MoveRight`
  (params (AxisValue :type "Float (single-precision)"))
  ;[1 1 1] 游戏开始与移动
  (if (`self.Start`)
    (`self.AddMovementInput` (0.0 -1.0 0.0))))

(event `Key|LeftMouseButton`
  (params (Key :type "Key Structure"))
  (bind _animinstance (`self.AnimInstance`))
  ;[1 1 1] Attack
  (:`Pressed`
    (`|PlayMontage` (`self.Mesh`) "/Game/Blueprints/Infinite/Anim_InfiniteLevels_Attack.Anim_InfiniteLevels_Attack"
      (:`then`
        (set `/Game/Anim/InfiniteLevels_AnimBP.IsAttack` true _animinstance))
      (:`OnCompleted`
        (set `/Game/Anim/InfiniteLevels_AnimBP.IsAttack` false _animinstance)))))

(event `Key|SpaceBar`
  (params (Key :type "Key Structure"))
  ;[1 1 1] 蹲下
  (:`Pressed`
    (`self.Crouch`))
  (:`Released`
    (`self.UnCrouch`)))

(fn `UserConstructionScript`)