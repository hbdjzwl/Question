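; BP_Wall is a breakable wall with pool-style push and pop events, showing a static wall mesh until it is broken.
; PopObject adds a fresh destructible component and reveals the mesh, and PushObject destroys that component.
; Broken hides the mesh, disables its collision, then reveals the destructible and applies heavy damage with an impulse in the supplied direction.
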(event `SimpleObjectPoolInterface.BP_PushObject`
  (bind _destructiblewall (`self.DestructibleWall`))
  (`/Engine/EditorBlueprintResources/StandardMacros.IsValid` _destructiblewall
    (:`Is Valid`
      (`ActorComponent.K2_DestroyComponent` _destructiblewall))))

(event `SimpleObjectPoolInterface.BP_PopObject`
  (bind _returnvalue (`AddComponent|NODE_AddDestructibleComponent-0`))
  (set `self.DestructibleWall` _returnvalue)
  (`SceneComponent.SetVisibility` (`self.WallMesh`) true false))

(event `SimpleObjectPoolInterface.BP_ObjectPreinitialized`)

(event `Broken`
  (params (ImpulseDir :type "Vector Structure (by ref)"))
  (bind _wallmesh (`self.WallMesh`))
  (bind _destructiblewall (`self.DestructibleWall`))
  (`PrimitiveComponent.SetCollisionEnabled` _wallmesh "NoCollision")
  (`SceneComponent.SetVisibility` _wallmesh false false)
  (`SceneComponent.SetVisibility` _destructiblewall true false)
  (`DestructibleComponent.ApplyDamage` _destructiblewall 8000.0 (`self.K2_GetActorLocation`) ImpulseDir 2500.0))

(fn `UserConstructionScript`)