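; Character Blueprint that plays montage-based key combos and shows the entered keys in a W_ComboMain widget.
; Valid keys build a string, looked up in Combo's array of maps indexed by sequence length.
; Finishers reset the string and open a gate to clear the widget on montage completion; misses reset after a short delay.
; Keys 1 and 2 print debug tables; an older DT_Combo-based implementation remains unconnected.
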(event `self.ReceiveBeginPlay`
  (bind _returnvalue (`|CreateWidget` "/Game/Blueprints/Combo/W_ComboMain.W_ComboMain_C"))
  (bind _output_get (set `self.ComboMain` _returnvalue))
  (`UserWidget.AddToViewport` _output_get 0))

(event `Key|One`
  (params (Key :type "Key Structure"))
  (:`Pressed`
    (for (_array_element _array_index) (`self.ArrayAttack`)
      (bind _keys (`BlueprintMapLibrary.Map_Keys` (break `/Game/Blueprints/Combo/NewFolder/S_ComboAttack` _array_element)))
      (bind _values (`BlueprintMapLibrary.Map_Values` (break `/Game/Blueprints/Combo/NewFolder/S_ComboAttack` _array_element)))
      (for (_array_element_2 _array_index_2) _keys
        (bind (_output_anim _output_finish) (break `/Game/Blueprints/Combo/NewFolder/S_AttackInfo` (`|GetArrayItem` _values _array_index_2)))
        (`KismetSystemLibrary.PrintString` (`KismetStringLibrary.Concat_StrStr` (`KismetStringLibrary.Conv_IntToString` _array_index) ":" _array_element_2 " ---- " (`KismetSystemLibrary.GetDisplayName` _output_anim) " ---- " (`KismetStringLibrary.Conv_BoolToString` _output_finish)) true true (struct :`R` 1.0 :`G` 0.537236 :`A` 1.0) 99.0)))))

(event `Key|Two`
  (params (Key :type "Key Structure"))
  (:`Pressed`
    (for (_array_element _array_index) (`ComboComponent.ComboAnimArray` (`self.Combo`))
      (bind _comboaniminfo (break `ComboAnim` _array_element))
      (bind _keys (`BlueprintMapLibrary.Map_Keys` _comboaniminfo))
      (bind _values (`BlueprintMapLibrary.Map_Values` _comboaniminfo))
      (for (_array_element_2 _array_index_2) _keys
        (bind (_animmontage _bfinish) (break `AnimInfo` (`|GetArrayItem` _values _array_index_2)))
        (`KismetSystemLibrary.PrintString` (`KismetStringLibrary.Concat_StrStr` (`KismetStringLibrary.Conv_IntToString` _array_index) ":" _array_element_2 "---" (`KismetSystemLibrary.GetDisplayName` _animmontage) "---" (`KismetStringLibrary.Conv_BoolToString` _bfinish)) true true (struct :`G` 1.0 :`A` 1.0) 99.0)))))

(event `Key|AnyKey`
  (params (Key :type "Key Structure"))
  (bind _combomain (`self.ComboMain`))
  (bind _combo (`self.Combo`))
  (:`Pressed`
    (if (`KismetArrayLibrary.Array_Contains` (`ComboComponent.InputKeys` _combo) Key)
      (bind _output_get (set `self.CurrentKeys` (`KismetStringLibrary.Concat_StrStr` (`self.CurrentKeys`) (`KismetTextLibrary.Conv_TextToString` (`KismetInputLibrary.Key_GetDisplayName` Key)))))
      (bind _returnvalue (`KismetStringLibrary.Len` _output_get))
      (`KismetSystemLibrary.PrintString` (`KismetStringLibrary.Concat_StrStr` (`KismetStringLibrary.Conv_IntToString` _returnvalue) ":" _output_get) true true (struct :`R` 1.0 :`G` 0.642559 :`A` 1.0) 5.0)
      (bind (_value _returnvalue_2) (`BlueprintMapLibrary.Map_Find` (`.ComboAnimInfo` (break `ComboAnim` (`|GetArrayItem` (`ComboComponent.ComboAnimArray` _combo) (- _returnvalue 1)))) _output_get))
      (if _returnvalue_2
        (`|PlayMontage` (`self.Mesh`) (break `AnimInfo` _value)
          (:`then`
            (`/Game/Blueprints/Combo/W_ComboMain.UpdateInputWidget` _combomain Key)
            (if (`.bFinish` (break `AnimInfo` _value))
              (set `self.CurrentKeys` "")
              (goto _label :!via `Open`)))
          (:`OnCompleted`
            (`/Engine/EditorBlueprintResources/StandardMacros.Gate` true :!label _label
              (:`Exit`
                (`/Game/Blueprints/Combo/W_ComboMain.ClearInputWidget` _combomain)
                (goto _label :!via `Close`)))))
        (else
          (`KismetSystemLibrary.Delay` 0.2)
          (`/Game/Blueprints/Combo/W_ComboMain.ClearInputWidget` _combomain)
          (set `self.CurrentKeys` "")
          (goto _label :!via `Close`))))))

(fn `UserConstructionScript`)