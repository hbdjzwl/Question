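; Character Blueprint prototyping a key-sequence combo attack system driven by DT_Combo.
; BeginPlay flattens each row into cumulative key-name prefixes, stored in per-step maps of montage and finish flag.
; Registered key presses extend the current string, whose length selects the map, assuming single-character key names.
; Matches play their montage; misses or finishers reset the string, and key 1 prints the table for debugging.
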(event `self.ReceiveBeginPlay`
  (bind _arrayattack (`self.ArrayAttack`))
  (bind _outrownames (`DataTableFunctionLibrary.GetDataTableRowNames` "/Game/Blueprints/Commo/DT_Combo.DT_Combo"))
  (for _array_element _outrownames
    (bind _returnvalue (`|GetDataTableRow` "/Game/Blueprints/Commo/DT_Combo.DT_Combo" _array_element)
      (:`then`
        (bind _animkey (break `/Game/Blueprints/Commo/S_AttackConfig` _returnvalue))
        (bind _keys (`BlueprintMapLibrary.Map_Keys` _animkey))
        (bind _values (`BlueprintMapLibrary.Map_Values` _animkey))
        (for (_array_element_2 _array_index) _keys
          (`KismetArrayLibrary.Array_AddUnique` (`self.AllKet`) _array_element_2)
          (bind _output_get (set `self.Keys` (`KismetStringLibrary.Concat_StrStr` (`self.Keys`) (`KismetTextLibrary.Conv_TextToString` (`KismetInputLibrary.Key_GetDisplayName` _array_element_2)))))
          (if (`KismetArrayLibrary.Array_IsValidIndex` _arrayattack _array_index)
            (bind (_output_anim _output_finish) (break `/Game/Blueprints/Commo/S_AttackInfo` (`|GetArrayItem` _values _array_index)))
            (bind _s_attackinfo (make `/Game/Blueprints/Commo/S_AttackInfo` _output_anim _output_finish))
            (`BlueprintMapLibrary.Map_Add` (`.AnimKey_11_ECC8457549D154AC450D388B47A55A7C` (break `/Game/Blueprints/Commo/S_ComboAttack` (`|GetArrayItem` _arrayattack _array_index))) _output_get _s_attackinfo)
            (else
              (`KismetArrayLibrary.Array_Set` _arrayattack _array_index (make `/Game/Blueprints/Commo/S_ComboAttack` (`|MakeMap` _output_get _s_attackinfo)) true))))
        (set `self.Keys` "")))))

(event `Key|One`
  (params (Key :type "Key Structure"))
  (:`Pressed`
    (for (_array_element _array_index) (`self.ArrayAttack`)
      (bind _keys (`BlueprintMapLibrary.Map_Keys` (break `/Game/Blueprints/Commo/S_ComboAttack` _array_element)))
      (bind _values (`BlueprintMapLibrary.Map_Values` (break `/Game/Blueprints/Commo/S_ComboAttack` _array_element)))
      (for (_array_element_2 _array_index_2) _keys
        (bind (_output_anim _output_finish) (break `/Game/Blueprints/Commo/S_AttackInfo` (`|GetArrayItem` _values _array_index_2)))
        (`KismetSystemLibrary.PrintString` (`KismetStringLibrary.Concat_StrStr` (`KismetStringLibrary.Conv_IntToString` _array_index) ":" _array_element_2 " ---- " (`KismetSystemLibrary.GetDisplayName` _output_anim) " ---- " (`KismetStringLibrary.Conv_BoolToString` _output_finish)) true true (struct :`R` 1.0 :`G` 0.537236 :`A` 1.0) 99.0)))))

(event `Key|AnyKey`
  (params (Key :type "Key Structure"))
  (:`Pressed`
    (if (`KismetArrayLibrary.Array_Contains` (`self.AllKet`) Key)
      (bind _output_get (set `self.CurrentKeys` (`KismetStringLibrary.Concat_StrStr` (`self.CurrentKeys`) (`KismetTextLibrary.Conv_TextToString` (`KismetInputLibrary.Key_GetDisplayName` Key)))))
      (bind _returnvalue (`KismetStringLibrary.Len` _output_get))
      (`KismetSystemLibrary.PrintString` (`KismetStringLibrary.Concat_StrStr` (`KismetStringLibrary.Conv_IntToString` _returnvalue) ":" _output_get) true true (struct :`R` 1.0 :`G` 0.642559 :`A` 1.0) 5.0)
      (bind (_value _returnvalue_2) (`BlueprintMapLibrary.Map_Find` (`.AnimKey_11_ECC8457549D154AC450D388B47A55A7C` (break `/Game/Blueprints/Commo/S_ComboAttack` (`|GetArrayItem` (`self.ArrayAttack`) (- _returnvalue 1)))) _output_get))
      (if _returnvalue_2
        (`|PlayMontage` (`self.Mesh`) (break `/Game/Blueprints/Commo/S_AttackInfo` _value)
          (:`then`
            (if (`.Finish_5_78D2E78F4DD8BB2D41DA6DB829C5C2AE` (break `/Game/Blueprints/Commo/S_AttackInfo` _value))
              (set `self.CurrentKeys` "" :!label _label))))
        (else
          (goto _label))))))

(fn `UserConstructionScript`)